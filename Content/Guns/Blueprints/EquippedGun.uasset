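; EquippedGun handles firing for the player's equipped gun, using the GunTable row named by GunName.
; BeginPlay caches the player and fills the magazine as temporary test setup.
; PlayerShoot requires aiming and ammo, delays the first shot, then runs a debug-drawn forward line trace whose hit is unused.
; A fire-rate gate resets automatically for "Auto" guns, otherwise on TriggerReleased once the delay completes.
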(event Custom|PlayerShoot
  (bind _player (Variables|Default|GetPlayer))
  (bind _shootpoint (Variables|/Game/ThirdPerson/Blueprints/BP_ThirdPersonCharacter.BP_ThirdPersonCharacter_C|GetShootPoint _player))
  (bind _returnvalue (Transformation|GetWorldLocation _shootpoint))
  ;[1 1 1] Shoot
  (bind _returnvalue_2 (Utilities|GetDataTableRow "/Game/Guns/Data/GunTable.GunTable" (Variables|Default|GetGunName))
    (:then
      (if (Math|Boolean|ANDBoolean (Variables|/Game/ThirdPerson/Blueprints/BP_ThirdPersonCharacter.BP_ThirdPersonCharacter_C|GetAiming _player) (not (Variables|Default|GetFireRateDelay)) (> (Variables|Default|GetShotsInMag) 0))
        (if (Variables|Default|GetFirstShot)
          (Utilities|FlowControl|Delay (.ShotDelay (Utilities|Struct|BreakGunStruct _returnvalue_2)))
          (Variables|Default|SetFirstShot false))
        (Collision|LineTraceByChannel _returnvalue (+ _returnvalue (* (Transformation|GetActorForwardVector _player) (Variables|Default|GetRange))) "TraceTypeQuery1" false 0 "ForDuration")
        (Math|Integer|DecrementInt (Variables|Default|GetShotsInMag)
          (:%20%20
            (Variables|Default|SetFireRateComplete false)
            (Variables|Default|SetFireRateDelay true)
            (Utilities|FlowControl|Delay (.FireRate (Utilities|Struct|BreakGunStruct _returnvalue_2)))
            (Variables|Default|SetFireRateComplete true)
            (if (Utilities|Enum|Equal(Enum) "Auto" (.Tag (Utilities|Struct|BreakGunStruct _returnvalue_2)))
              (Variables|Default|SetFireRateDelay false))))))))

(event Custom|TriggerReleased
  ;[1 1 1] Trigger Released
  (Variables|Default|SetFirstShot true)
  (if (Variables|Default|GetFireRateComplete)
    (Variables|Default|SetFireRateDelay false)))

(event EventBeginPlay
  ;[1 1 1] Begin Play
  (Variables|Default|SetOwner (Components|GetOwner))
  (bind _asbp_third_person_character (Utilities|Casting|CastToBP_ThirdPersonCharacter (Game|GetPlayerCharacter 0)))
  (Variables|Default|SetPlayer _asbp_third_person_character)
  ;[1 1 1] FOR TESTING - DELETE
  (bind _returnvalue (Utilities|GetDataTableRow "/Game/Guns/Data/GunTable.GunTable" (Variables|Default|GetGunName))
    (:then
      (Variables|Default|SetShotsInMag (.MagSize (Utilities|Struct|BreakGunStruct _returnvalue))))))