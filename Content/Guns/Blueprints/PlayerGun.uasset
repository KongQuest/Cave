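; Player gun Blueprint that fires a debug-drawn line trace from the character's shoot point along its forward vector while aiming.
; It looks up the gun's row in a data table by name for fire rate and tag, locking firing during the delay.
; "Auto" guns unlock after the delay, while others need a trigger release once it completes.
; The trace result is not used, so no damage is applied here.
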(event Custom|PlayerShoot
  (bind _player (Variables|Default|GetPlayer))
  (bind _shootpoint (Variables|/Game/ThirdPerson/Blueprints/BP_ThirdPersonCharacter.BP_ThirdPersonCharacter_C|GetShootPoint _player))
  (bind _returnvalue (Transformation|GetWorldLocation _shootpoint))
  ;[1 1 1] Shoot
  (bind _returnvalue_2 (Utilities|GetDataTableRow "/Game/Guns/Data/GunTable.GunTable" (Variables|Default|GetGunName))
    (:then
      (if (and (Variables|/Game/ThirdPerson/Blueprints/BP_ThirdPersonCharacter.BP_ThirdPersonCharacter_C|GetAiming _player) (not (Variables|Default|GetCannotFire)))
        (Collision|LineTraceByChannel _returnvalue (+ _returnvalue (* (Transformation|GetActorForwardVector _player) (Variables|Default|GetRange))) "TraceTypeQuery1" false 0 "ForDuration")
        (Variables|Default|SetFireRateComplete false)
        (Variables|Default|SetCannotFire true)
        (Utilities|FlowControl|Delay (.FireRate (Utilities|Struct|BreakGunRow _returnvalue_2)))
        (Variables|Default|SetFireRateComplete true)
        (if (Utilities|Enum|Equal(Enum) "Auto" (.Tag (Utilities|Struct|BreakGunRow _returnvalue_2)))
          (Variables|Default|SetCannotFire false))))))

(event Custom|TriggerReleased
  ;[1 1 1] Trigger Released
  (if (Variables|Default|GetFireRateComplete)
    (Variables|Default|SetCannotFire false)))

(event EventBeginPlay
  ;[1 1 1] Begin Play
  (Variables|Default|SetOwner (Components|GetOwner))
  (bind _asbp_third_person_character (Utilities|Casting|CastToBP_ThirdPersonCharacter (Game|GetPlayerCharacter 0)))
  (Variables|Default|SetPlayer _asbp_third_person_character))